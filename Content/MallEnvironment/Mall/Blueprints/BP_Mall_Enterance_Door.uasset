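; Mall entrance door Blueprint that swings open when a Character enters either of its two trigger volumes.
; The Left and Right triggers each play their own Timeline, lerping the door mesh's relative yaw a quarter turn in opposite directions.
; LeftOpen and RightOpen flags block opening in one direction while the other is active.
; A fixed three-second Delay after overlap clears the flag and reverses that Timeline to close the door.
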(event OnComponentBeginOverlap(Left)
  (params (OverlappedComponent :type Primitive%20Component%20Object%20Reference) (OtherActor :type Actor%20Object%20Reference) (OtherComp :type Primitive%20Component%20Object%20Reference) (OtherBodyIndex :type Integer) (bFromSweep :type Boolean) (SweepResult :type Hit%20Result%20Structure%20%28by%20ref%29))
  ;[1 1 1] Left trigger (Close door after 3 sec)
  (Utilities|Casting|CastToCharacter OtherActor)
  (CallFunction|LeftOpenEvent)
  (Utilities|FlowControl|Delay 3.0)
  (CallFunction|LeftCloseEvent))

(event OnComponentBeginOverlap(Right)
  (params (OverlappedComponent :type Primitive%20Component%20Object%20Reference) (OtherActor :type Actor%20Object%20Reference) (OtherComp :type Primitive%20Component%20Object%20Reference) (OtherBodyIndex :type Integer) (bFromSweep :type Boolean) (SweepResult :type Hit%20Result%20Structure%20%28by%20ref%29))
  ;[1 1 1] Right trigger (Close door after 3 sec)
  (Utilities|Casting|CastToCharacter OtherActor)
  (CallFunction|RightOpenEvent)
  (Utilities|FlowControl|Delay 3.0)
  (CallFunction|RightCloseEvent))

(event Custom|RightOpenEvent
  ;[1 1 1] Open - Close Door to Right
  (if (not (Variables|Default|GetLeftOpen))
    (Variables|Default|SetRightOpen true)
    (bind _alpha (Timeline|Timeline_1 Play)
      (:Update
        (Transformation|SetRelativeRotation (Variables|Default|GetSM_Mall_Enterance_Door) (Math|Rotator|MakeRotator 0.0 0.0 (Math|Float|Lerp 0.0 9e+01 _alpha)) false false)))))

(event Custom|RightCloseEvent
  ;[1 1 1] Open - Close Door to Right
  (Variables|Default|SetRightOpen false)
  (bind _alpha (Timeline|Timeline_1 Reverse)
    (:Update
      (Transformation|SetRelativeRotation (Variables|Default|GetSM_Mall_Enterance_Door) (Math|Rotator|MakeRotator 0.0 0.0 (Math|Float|Lerp 0.0 9e+01 _alpha)) false false))))

(event Custom|LeftOpenEvent
  ;[1 1 1] Open - Close Door to left
  (if (not (Variables|Default|GetRightOpen))
    (Variables|Default|SetLeftOpen true)
    (bind _alpha (Timeline|Timeline_0 Play)
      (:Update
        (Transformation|SetRelativeRotation (Variables|Default|GetSM_Mall_Enterance_Door) (Math|Rotator|MakeRotator 0.0 0.0 (Math|Float|Lerp 0.0 -9e+01 _alpha)) false false)))))

(event Custom|LeftCloseEvent
  ;[1 1 1] Open - Close Door to left
  (Variables|Default|SetLeftOpen false)
  (bind _alpha (Timeline|Timeline_0 Reverse)
    (:Update
      (Transformation|SetRelativeRotation (Variables|Default|GetSM_Mall_Enterance_Door) (Math|Rotator|MakeRotator 0.0 0.0 (Math|Float|Lerp 0.0 -9e+01 _alpha)) false false))))

(fn ConstructionScript)