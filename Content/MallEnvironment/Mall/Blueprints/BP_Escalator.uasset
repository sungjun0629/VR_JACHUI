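; BP_Escalator is an escalator for the mall environment with animated stairs that travel along a spline.
; The construction script picks the forward or reverse spline and adds stair meshes along it at StepDistance intervals, recording each one's distance.
; When Active, a looping timer started at BeginPlay advances each step by Speed, updating only its location and resetting its distance at the spline's end for continuous motion.
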(event Custom|MoveStairs
  (bind _current_distance (Variables|Default|GetCurrent_Distance))
  ;[1 1 1] Run stairs if active is selected
  (for (_array_element _array_index) (Variables|Default|GetSteps)
    (Transformation|SetWorldLocation _array_element (Spline|GetLocationatDistanceAlongSpline (Variables|Default|GetDirection) (Utilities|Array|Get(acopy) _current_distance _array_index) "World") false false)
    (Math|Float|CompareFloat (+ (Utilities|Array|Get(acopy) _current_distance _array_index) (Variables|Default|GetSpeed)) (Spline|GetSplineLength (Variables|Default|GetDirection))
      (:>
        (Utilities|Array|SetArrayElem _current_distance _array_index 0.0 true))
      (:<
        (Utilities|Array|SetArrayElem _current_distance _array_index (+ (Utilities|Array|Get(acopy) _current_distance _array_index) (Variables|Default|GetSpeed)) true)))))

(event EventBeginPlay
  ;[1 1 1] Run stairs if active is selected
  (if (Variables|Default|GetActive)
    (Utilities|Time|SetTimerbyEvent (delegate Custom|MoveStairs) 0.01 true)))

(fn ConstructionScript
  (bind _step_distance (Variables|Default|GetStep_Distance))
  (if (Variables|Default|GetReverse?)
    (Variables|Default|SetDirection (Variables|Default|GetReverse))
    (else
      (Variables|Default|SetDirection (Variables|Default|GetSpline))))
  (for _index (range 0 (.ReturnValue (Math|Float|Division(WholeandRemainder) (Spline|GetSplineLength (Variables|Default|GetDirection)) _step_distance)))
    (Utilities|Array|Add (Variables|Default|GetCurrent_Distance) (* _index _step_distance))
    (bind _returnvalue (AddComponent|AddStaticMeshComponent false (Math|Transform|MakeTransform (Spline|GetLocationatDistanceAlongSpline (Variables|Default|GetDirection) (* _index _step_distance) "World") "0,90.000000, 0")))
    (Components|StaticMesh|SetStaticMesh _returnvalue "/Game/MallEnvironment/Mall/Meshes/Escalator/SM_Escalator_Stair.SM_Escalator_Stair")
    (Utilities|Array|Add (Variables|Default|GetSteps) _returnvalue)))