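; Mall entrance Blueprint with two sliding doors that open automatically when a Character steps into its trigger volume.
; BeginPlay stores each door's starting X, and a timeline lerps both apart by DoorOpenValue.
; Leaving the trigger reverses the timeline after a short delay, unless the OnDoor flag shows a Character has re-entered by then.
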(event OnComponentBeginOverlap(Trigger)
  (params (OverlappedComponent :type Primitive%20Component%20Object%20Reference) (OtherActor :type Actor%20Object%20Reference) (OtherComp :type Primitive%20Component%20Object%20Reference) (OtherBodyIndex :type Integer) (bFromSweep :type Boolean) (SweepResult :type Hit%20Result%20Structure%20%28by%20ref%29))
  ;[1 1 1] Trigger
  (Utilities|Casting|CastToCharacter OtherActor)
  (Variables|Default|SetOnDoor true)
  (CallFunction|OpenEvent))

(event OnComponentEndOverlap(Trigger)
  (params (OverlappedComponent :type Primitive%20Component%20Object%20Reference) (OtherActor :type Actor%20Object%20Reference) (OtherComp :type Primitive%20Component%20Object%20Reference) (OtherBodyIndex :type Integer))
  ;[1 1 1] Trigger
  (Utilities|Casting|CastToCharacter OtherActor)
  (Variables|Default|SetOnDoor false)
  (Utilities|FlowControl|Delay 3.0)
  (CallFunction|CloseEvent))

(event Custom|OpenEvent
  ;[1 1 1] Open - Close Door
  (if (Variables|Default|GetOnDoor)
    (if (not (Variables|Default|GetOpen))
      (Variables|Default|SetOpen true)
      (bind _alpha (Timeline|Timeline_0 Play)
        (:Update
          (Transformation|SetRelativeLocation (Variables|Default|GetSM_SlidingDoorL) (Math|Vector|MakeVector (Math|Float|Lerp (Variables|Default|GetLstart) (- (Variables|Default|GetLstart) (Variables|Default|GetDoor_Open_Value)) _alpha) 13.0 0.0) false false)
          (Transformation|SetRelativeLocation (Variables|Default|GetSM_SlidingDoorR) (Math|Vector|MakeVector (Math|Float|Lerp (Variables|Default|GetRstart) (+ (Variables|Default|GetRstart) (Variables|Default|GetDoor_Open_Value)) _alpha) 13.0 0.0) false false))))))

(event Custom|CloseEvent
  ;[1 1 1] Open - Close Door
  (if (not (Variables|Default|GetOnDoor))
    (Variables|Default|SetOpen false)
    (bind _alpha (Timeline|Timeline_0 Reverse)
      (:Update
        (Transformation|SetRelativeLocation (Variables|Default|GetSM_SlidingDoorL) (Math|Vector|MakeVector (Math|Float|Lerp (Variables|Default|GetLstart) (- (Variables|Default|GetLstart) (Variables|Default|GetDoor_Open_Value)) _alpha) 13.0 0.0) false false)
        (Transformation|SetRelativeLocation (Variables|Default|GetSM_SlidingDoorR) (Math|Vector|MakeVector (Math|Float|Lerp (Variables|Default|GetRstart) (+ (Variables|Default|GetRstart) (Variables|Default|GetDoor_Open_Value)) _alpha) 13.0 0.0) false false)))))

(event EventBeginPlay
  (Variables|Default|SetLstart (.x (Variables|/Script/Engine.SceneComponent|GetRelativeLocation (Variables|Default|GetSM_SlidingDoorL))))
  (Variables|Default|SetRstart (.x (Variables|/Script/Engine.SceneComponent|GetRelativeLocation (Variables|Default|GetSM_SlidingDoorR)))))

(fn ConstructionScript)